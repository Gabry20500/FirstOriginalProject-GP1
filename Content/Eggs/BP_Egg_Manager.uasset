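; BP_Egg_Manager spawns sets of BP_Egg actors at randomly chosen BP_Egg_TargetPoint locations in the level.
; On BeginPlay it gathers the target points and spawns three eggs, each slightly below a random point, counting them in EggInScene.
; DecreaseEggs lowers that count and spawns a new set after a short delay when it reaches zero.
; The TakenSpots duplicate check is disconnected, so eggs can share a spot.
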(event Custom|SpawnEggSet
  (for _index (range 0 2)
    (Variables|Default|SetActualSpot (Math|Random|RandomIntegerinRange 0 (- (Utilities|Array|Length (Variables|Default|GetTargetPointsArr)) 1)))
    (CallFunction|IncreaseEgg)
    (Game|SpawnActorfromClass "/Game/Eggs/BP_Egg.BP_Egg_C" (Math|Transform|MakeTransform (- (Transformation|GetActorLocation (Utilities|Array|Get(acopy) (Variables|Default|GetTargetPointsArr) (Variables|Default|GetActualSpot))) "0, 0,100.000000") "0, 0, 0" "1,1,1") "Undefined" 0 0))
  (Utilities|Array|Clear (Variables|Default|GetTakenSpots)))

(event Custom|IncreaseEgg
  (Variables|Default|SetEggInScene (+ (Variables|Default|GetEggInScene) 1)))

(event Custom|DecreaseEggs
  (Variables|Default|SetEggInScene (- (Variables|Default|GetEggInScene) 1))
  (if (== (Variables|Default|GetEggInScene) 0)
    (Utilities|FlowControl|Delay 1.0)
    (CallFunction|SpawnEggSet)))

(event EventBeginPlay
  (bind _outactors (Actor|GetAllActorsOfClass "/Game/TargetPoint/BP_Egg_TargetPoint.BP_Egg_TargetPoint_C"))
  (Variables|Default|SetTargetPointsArr _outactors)
  (CallFunction|SpawnEggSet))

(fn ConstructionScript)