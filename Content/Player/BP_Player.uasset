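; Player character, a honey badger that moves in short hops, keeps a score and dies when hit by a projectile.
; Forward and side axis inputs launch it along fixed world axes with an upward kick, gated by a brief cooldown.
; An overlap with BP_Projectile calls Death, which disables movement, swaps the mesh and shows the death screen with cursor.
; After a delay, the mesh becomes a soul and the capsule floats upward.
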(event OnComponentBeginOverlap(CollisionBox)
  (params (OverlappedComponent :type Primitive%20Component%20Object%20Reference) (OtherActor :type Actor%20Object%20Reference) (OtherComp :type Primitive%20Component%20Object%20Reference) (OtherBodyIndex :type Integer) (bFromSweep :type Boolean) (SweepResult :type Hit%20Result%20Structure%20%28by%20ref%29))
  (bind _capsulecomponent (Variables|Collision|GetCapsuleComponent))
  ;[1 1 1] Death
  (if (== (Utilities|GetClass OtherActor) "/Game/ShootingSystem/BP_Projectile.BP_Projectile_C")
    (CallFunction|Death)
    (Utilities|FlowControl|Delay 1.0)
    (Components|StaticMesh|SetStaticMesh (Variables|Default|GetCube) "/Game/3D_Assets/Cartons_Honey_badger_soul.Cartons_Honey_badger_soul")
    (Components|MoveComponentTo _capsulecomponent (+ (Transformation|GetWorldLocation _capsulecomponent) "0, 0,800.000000") "0, 0, 0" false false 2.0 false)))

(event Custom|MovementCooldown
  ;[1 1 1] Create delay for movement
  (Variables|Default|SetCanMove false)
  (Utilities|FlowControl|Delay 0.4)
  (Variables|Default|SetCanMove true))

(event Custom|IncreaseScore
  ;[1 1 1] Increase Score
  (Variables|Default|SetScore (+ (Variables|Default|GetScore) 1)))

(event Input|AxisEvents|InputAxisMoveForeward
  (params (AxisValue :type Float%20%28single-precision%29))
  ;[1 1 1] Movement
  (Variables|Default|SetForeWardValue AxisValue)
  (if (and (!= AxisValue 0.0) (Variables|Default|GetCanMove))
    (Utilities|FlowControl|Sequence
      (:then_0
        (if (!= (Variables|Default|GetForeWardValue) 0.0)
          (Variables|Default|SetMultiplyValue (* (Variables|Default|GetForeWardValue) -2.5e+02))
          (else
            (Variables|Default|SetMultiplyValue (* (Variables|Default|GetForeWardValue) 2.5e+02)))))
      (:then_1
        (CallFunction|MovementCooldown)
        (Character|LaunchCharacter (Math|Vector|MakeVector (Variables|Default|GetMultiplyValue) 0.0 2e+02) true true)))))

(event Input|AxisEvents|InputAxisMoveSide
  (params (AxisValue :type Float%20%28single-precision%29))
  ;[1 1 1] Movement
  (bind _output_get (Variables|Default|SetSideValue AxisValue))
  (if (and (!= _output_get 0.0) (Variables|Default|GetCanMove))
    (Utilities|FlowControl|Sequence
      (:then_0
        (if (!= (Variables|Default|GetSideValue) 0.0)
          (Variables|Default|SetMultiplyValue (* (Variables|Default|GetSideValue) -2.5e+02))
          (else
            (Variables|Default|SetMultiplyValue (* (Variables|Default|GetSideValue) 2.5e+02)))))
      (:then_1
        (CallFunction|MovementCooldown)
        (Character|LaunchCharacter (Math|Vector|MakeVector 0.0 (Variables|Default|GetMultiplyValue) 2e+02) true true)))))

(fn ConstructionScript)

(fn Death
  ;[1 1 1] Player Is Dead
  (bind _returnvalue (UserInterface|CreateWidget "/Game/Player/WG_DeathScreen.WG_DeathScreen_C"))
  (UserInterface|Viewport|AddtoViewport _returnvalue 0)
  (Pawn|Components|CharacterMovement|DisableMovement (Variables|Character|GetCharacterMovement))
  (Components|StaticMesh|SetStaticMesh (Variables|Default|GetCube) "/Game/3D_Assets/Cartons_Honey_badger_death.Cartons_Honey_badger_death")
  (Variables|/Script/Engine.PlayerController|SetbShowMouseCursor (Game|GetPlayerController 0) true))